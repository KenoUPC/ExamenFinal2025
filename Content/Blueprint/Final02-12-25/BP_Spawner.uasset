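; BP_Spawner is an actor that toggles the creation of actors on and off through its Activar event.
; Each call flips the Activado flag, either telling its BPCActivableComponent to start creating actors at the spawner's transform or to stop.
; The spawning logic lives in that component, and the spawner prints the new state as debug text.
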(event `/Game/Blueprint/Final02-12-25/BPI_Interactuables.Activar`
  (if (not (`self.bActivado?`))
    (`/Game/Blueprint/Final02-12-25/BP_ActivableComponent.ComiezoACrearActores` (`self.BPC_ActivableComponent`) (`self.GetTransform`))
    (set `self.bActivado?` true)
    (`KismetSystemLibrary.PrintString` "Activado")
    (else
      (`/Game/Blueprint/Final02-12-25/BP_ActivableComponent.PararConLaCreacion` (`self.BPC_ActivableComponent`))
      (set `self.bActivado?` false)
      (`KismetSystemLibrary.PrintString` "Desactivado"))))

(fn `UserConstructionScript`)