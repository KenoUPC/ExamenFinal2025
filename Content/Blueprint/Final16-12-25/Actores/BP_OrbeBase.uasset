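; BP_OrbeBase is an orb actor, apparently a base class, that can be picked up as an element through interaction.
; Its widget starts hidden and is shown or hidden as any actor begins or ends overlap.
; Interact passes the orb to TryPickupElement on the interacting actor's BPC_ElementCarrier, prints a debug message, then destroys the orb without checking whether the pickup succeeded.
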(event `self.ReceiveBeginPlay`
  (`SceneComponent.SetVisibility` (`self.Widget`) false false))

(event `self.ReceiveActorBeginOverlap`
  (params (OtherActor :type "Actor Object Reference"))
  (`SceneComponent.SetVisibility` (`self.Widget`) true false))

(event `self.ReceiveActorEndOverlap`
  (params (OtherActor :type "Actor Object Reference"))
  (`SceneComponent.SetVisibility` (`self.Widget`) false false))

(event `/Game/Blueprint/Final16-12-25/Blueprtinrs/BP_Interact16-12.Interact`
  (params (Actor :type "Actor Object Reference"))
  (`/Game/Blueprint/Final16-12-25/Blueprtinrs/BPC_ElementCarrier.TryPickupElement` (`self.GetComponentByClass` Actor "/Game/Blueprint/Final16-12-25/Blueprtinrs/BPC_ElementCarrier.BPC_ElementCarrier_C") self)
  (`KismetSystemLibrary.PrintString` "Preguntando al compoenete")
  (`self.K2_DestroyActor`))

(fn `UserConstructionScript`)