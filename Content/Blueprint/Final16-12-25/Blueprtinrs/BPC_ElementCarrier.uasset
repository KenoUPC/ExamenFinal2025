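; BPC_ElementCarrier is a component that tracks which elemental orb type its owner carries, and how many.
; TryPickupElement increments the count for a matching type or the NewEnumerator4 state, remembering the orb's class.
; A different type respawns the held orbs from that class in a row along X beside the owner, then restarts the count at one.
; CheckElement returns type and count, zeroing only the count.
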(fn `CheckElement`
  (returns (CurrentElementType :type "/Game/Blueprint/Final16-12-25/Blueprtinrs/E_ElementType Enum") (CountCurrentType :type Integer))
  (bind _output_get (set `self.OutCurrentElemente` (`self.CountCurrentType`)))
  (set `self.CountCurrentType` 0)
  (return (`self.CurrentElementType`) _output_get))

(fn `TryPickupElement`
  (params (Element :type "/Game/Blueprint/Final16-12-25/Actores/BP_OrbeBase Object Reference"))
  (locals (NewLocalVar :type "Vector Structure" :default (0.0 0.0 0.0)))
  (bind _returnvalue (`GameplayStatics.GetObjectClass` Element))
  (bind _type (`/Game/Blueprint/Final16-12-25/Actores/BP_OrbeBase.Type` Element))
  (bind (_spawnpos_x _spawnpos_y _spawnpos_z) (`KismetMathLibrary.BreakVector` (`self.SpawnPos`)))
  (set `self.CurrentClass` _returnvalue)
  (`/Engine/EditorBlueprintResources/StandardMacros.IsValid` Element
    (:`Is Valid`
      (if (or (`|EnumEquality` _type (`self.CurrentElementType`)) (`|EnumEquality` (`self.CurrentElementType`) "NewEnumerator4"))
        (set `self.PreClass` _returnvalue)
        (bind _result (`/Engine/EditorBlueprintResources/StandardMacros.IncrementInt` (`self.CountCurrentType`))
          (:`  `
            (bind _output_get (set `self.CurrentElementType` _type))
            (`KismetSystemLibrary.PrintString` (`KismetStringLibrary.Concat_StrStr` "El tipo de Orbe es" (`|GetEnumeratorNameAsString` _output_get) " y tenes: \n" (`KismetStringLibrary.Conv_IntToString` _result)))))
        (else
          (set `self.CurrentElementType` _type)
          (set `self.SpawnPos` (`Actor.K2_GetActorLocation` (`self.GetOwner`)))
          (`KismetSystemLibrary.PrintString` "es distinto")
          (for _ (range (`self.CountCurrentType`))
            (bind _output_get_2 (set `self.SpawnPos` (`KismetMathLibrary.MakeVector` (+ _spawnpos_x 50.0) _spawnpos_y _spawnpos_z)))
            (`|SpawnActorFromClass` (`self.PreClass`) (`KismetMathLibrary.MakeTransform` _output_get_2) "Undefined" "MultiplyWithRoot" null null))
          (set `self.CountCurrentType` 1)
          (set `self.PreClass` (`self.CurrentClass`)))))))